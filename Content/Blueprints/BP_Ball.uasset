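; BP_Ball is a ball that moves along its Direction at Speed and bounces off whatever blocks it.
; Tick moves it with a swept offset; on a blocking hit it reflects Direction and zeroes Z to keep movement horizontal.
; Each bounce subtracts a fixed step, computed at BeginPlay as a percentage of starting Speed, never dropping below MinSpeed.
; RoundTo snaps speed values to the precision set by the Numbers multiplier.
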(event EventBeginPlay
  (bind _returnvalue (CallFunction|Roundto (* (Math|Float|NormalizetoRange (Variables|Default|GetPercent) 0.0 1e+02) (Variables|Public|GetSpeed))))
  (Variables|Default|SetDeltaSpeed _returnvalue))

(event Collision|EventActorBeginOverlap
  (params (OtherActor :type Actor%20Object%20Reference)))

(event EventTick
  (params (DeltaSeconds :type Float%20%28single-precision%29))
  (bind _minspeed (Variables|Public|GetMinSpeed))
  (bind _sweephitresult (Transformation|AddActorWorldOffset (* (* (Variables|Default|GetDirection) (Variables|Public|GetSpeed)) DeltaSeconds) true))
  (if (.bblockinghit _sweephitresult)
    (Variables|Default|SetDirection (Math|Vector|MakeVector (.x (Math|Vector|GetReflectionVector (Variables|Default|GetDirection) (.normal _sweephitresult))) (.y (Math|Vector|GetReflectionVector (Variables|Default|GetDirection) (.normal _sweephitresult))) 0.0))
    (bind _returnvalue (CallFunction|Roundto (- (Variables|Public|GetSpeed) (Variables|Default|GetDeltaSpeed))))
    (if (>= _returnvalue _minspeed)
      (Variables|Public|SetSpeed _returnvalue)
      (else
        (Variables|Public|SetSpeed _minspeed)))))

(fn ConstructionScript)

(fn Roundto
  (params (Value :type Float%20%28single-precision%29))
  (bind _numbers (Variables|Default|GetNumbers))
  (return (/ (Math|Conversions|ToFloat(Integer) (Math|Float|Round (* _numbers Value))) (Math|Conversions|ToFloat(Integer) _numbers))))