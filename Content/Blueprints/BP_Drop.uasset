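; BP_Drop is a moving drop actor with a random type: New Ball, Reducing Size or Increasing Size.
; The construction script rolls the E_DropState from the enum's entry count, prints it, and assigns the cube a material matching that type.
; Tick moves it with a swept offset along Direction at Speed, and overlapping a KillZVolume destroys it.
; The type's gameplay effect is not applied here.
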(event EventBeginPlay)

(event Collision|EventActorBeginOverlap
  (params (OtherActor :type Actor%20Object%20Reference))
  (Utilities|Casting|CastToKillZVolume OtherActor)
  (Actor|DestroyActor))

(event EventTick
  (params (DeltaSeconds :type Float%20%28single-precision%29))
  (Transformation|AddActorWorldOffset (* (* (Variables|Default|GetDirection) (Variables|Default|GetSpeed)) DeltaSeconds) true))

(fn ConstructionScript
  (bind _cube (Variables|Default|GetCube))
  (bind _output_get (Variables|Default|SetDropState (Utilities|Enum|ByteToEnumE_DropState (Math|Conversions|ToByte(Integer) (Math|Random|RandomInteger (|GetNumEnumEntries))))))
  (Development|PrintString (Utilities|String|Append "Create Drop with: " (Utilities|String|EnumtoString _output_get)) true true "(R=0.209979,G=1.000000,B=0.192171,A=1.000000)" 5.0)
  (switch Utilities|FlowControl|Switch|SwitchonE_DropState _output_get
    (:NewEnumerator0
      (Rendering|Material|SetMaterial _cube 0 "/Game/StarterContent/Materials/M_Metal_Gold.M_Metal_Gold"))
    (:NewEnumerator1
      (Rendering|Material|SetMaterial _cube 0 "/Game/StarterContent/Materials/M_Metal_Copper.M_Metal_Copper"))
    (:NewEnumerator2
      (Rendering|Material|SetMaterial _cube 0 "/Game/StarterContent/Materials/M_Water_Ocean.M_Water_Ocean"))))